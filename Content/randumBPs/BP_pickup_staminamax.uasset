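; Stamina upgrade pickup that permanently raises the collecting character's maximum stamina.
; Its Pickup event casts the character's controller to ThirdPersonPlayerController and increases max stamina by a fixed amount, leaving max health unchanged.
; It then adds the same amount to the character's current stamina; nothing happens if the cast fails.
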(event EventBeginPlay
  (|CallParentFunction) ; This node is disabled and will not be called.\nDrag off pins to build functionality.
)

(event Collision|EventActorBeginOverlap
  (params (OtherActor :type Actor%20Object%20Reference))
  (|CallParentFunction OtherActor) ; This node is disabled and will not be called.\nDrag off pins to build functionality.
)

(event EventPickup
  (params (character :type Third%20Person%20Character%20Object%20Reference))
  (bind _asthird_person_player_controller (Utilities|Casting|CastToThirdPersonPlayerController (Pawn|GetController character)))
  (Default|IncreaseMaxHealthStamina _asthird_person_player_controller 0.0 25.0)
  (Default|ChangeHealthStamina character 0.0 25.0))

(event EventTick
  (params (DeltaSeconds :type Float%20%28single-precision%29))
  (|CallParentFunction DeltaSeconds) ; This node is disabled and will not be called.\nDrag off pins to build functionality.
)

(fn ConstructionScript
  (|CallParentFunction))